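; Effect object that applies one Health or Movement Speed effect to an AttributeComponent and shows a matching widget message.
; Untimed effects only handle Health, changing it once.
; Timed Health effects repeat the change on a looping timer until the duration is reached, while Movement Speed changes once and resets on expiry.
; When finished, it removes its widget and fires OnReadyForDelete so its owner can discard it.
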(event `ActivateEffect`
  (params (Settings :type "/Game/Core/Effect/Structure/S_EffectStructure Structure"))
  ;[1 1 1] StartEffect
  (bind _output_get (set `self.Settings` Settings))
  (`self.SetEffectWidget`)
  (if (not (`.NeedTimer_8_D00D3DF643B06BA6DEE8E98B0EE6B49C` (break `/Game/Core/Effect/Structure/S_EffectStructure` _output_get)))
    (`self.SimpleEffect`)
    (else
      (`self.EffectWithTimer`))))

(event `EffectWithTimer`
  (bind _settings_attribute (break `/Game/Core/Effect/Structure/S_EffectStructure` (`self.Settings`)))
  ;[1 1 1] SimpleAndWithTimer
  (switch `/Game/Core/Effect/Enum/E_AttributeSetting` _settings_attribute
    (:`NewEnumerator0`
      (`self.SetTimerHealth`))
    (:`NewEnumerator1`
      (`self.SetTimerMovementSpeed`))))

(event `SimpleEffect`
  (bind _settings_attribute (break `/Game/Core/Effect/Structure/S_EffectStructure` (`self.Settings`)))
  (bind (_settings_attribute_2 _settings_needtimer _settings_time _settings_damage) (break `/Game/Core/Effect/Structure/S_EffectStructure` (`self.Settings`)))
  ;[1 1 1] SimpleAndWithTimer
  (switch `/Game/Core/Effect/Enum/E_AttributeSetting` _settings_attribute
    (:`NewEnumerator0`
      (`self.HealthDamage` _settings_damage)
      (`self.PrepareForDelete`))))

(event `SetEffectWidget`
  (bind _settings_attribute (break `/Game/Core/Effect/Structure/S_EffectStructure` (`self.Settings`)))
  ;[1 1 1] Widget
  (bind _effectwidget (message `/Game/Widget/Interface/BI_SetNewWidgetEffect.SetNewWidgetEffect` (`WidgetComponent.GetWidget` (`self.EffectsWidget`)) _settings_attribute))
  (set `self.Effect Widget` _effectwidget))

(event `MovementSpeedDamage`
  (params (Damage :type "Float (double-precision)"))
  ;[1 1 1] MovementSpeed
  (bind _attributecomponent (`self.AttributeComponent`)
    (:`then`
      (`/Game/Core/Character/Components/BP_AttributeComponent.MovementSpeedChange` _attributecomponent Damage))
    (:`else`)))

(event `ResetMovementSpeed`
  ;[1 1 1] MovementSpeed
  (bind _attributecomponent (`self.AttributeComponent`)
    (:`then`
      (`/Game/Core/Character/Components/BP_AttributeComponent.ResetMovementSpeed` _attributecomponent))
    (:`else`)))

(event `PrepareForDelete`
  ;[1 1 1] PrepareForDelete
  (`self.RemoveWidget`)
  (if (`KismetSystemLibrary.K2_IsValidTimerHandle` (`self.Timer`))
    (`KismetSystemLibrary.K2_InvalidateTimerHandle` (`self.Timer`))
    (set `self.Timer` (struct)))
  (`self.OnReadyForDelete` self))

(event `SetTimerMovementSpeed`
  (bind (_settings_attribute _settings_needtimer _settings_time) (break `/Game/Core/Effect/Structure/S_EffectStructure` (`self.Settings`)))
  (bind (_settings_attribute_2 _settings_needtimer_2 _settings_time_2 _settings_damage) (break `/Game/Core/Effect/Structure/S_EffectStructure` (`self.Settings`)))
  ;[1 1 1] MovementSpeed
  (bind _returnvalue (`KismetSystemLibrary.K2_SetTimerDelegate` (delegate `TimerMovementSpeedBody`) _settings_time))
  (set `self.Timer` _returnvalue)
  (`self.MovementSpeedDamage` _settings_damage))

(event `InvalidedTimer`
  ;[1 1 1] PrepareForDelete
  (`KismetSystemLibrary.K2_InvalidateTimerHandle` (`self.Timer`))
  (set `self.Timer` (struct)))

(event `TimerMovementSpeedBody`
  ;[1 1 1] MovementSpeed
  (`self.InvalidedTimer`)
  (`self.ResetMovementSpeed`)
  (`self.RemoveWidget`)
  (`self.OnReadyForDelete` self))

(event `RemoveWidget`
  ;[1 1 1] PrepareForDelete
  (`Widget.RemoveFromParent` (`self.Effect Widget`)))

(event `SetAttributeComponent`
  (params (AttributeComponent :type "/Game/Core/Character/Components/BP_AttributeComponent Object Reference"))
  ;[1 1 1] Setters
  (set `self.AttributeComponent` AttributeComponent))

(event `HealthDamage`
  (params (Damage :type "Float (double-precision)"))
  ;[1 1 1] Health
  (bind _attributecomponent (`self.AttributeComponent`)
    (:`then`
      (`/Game/Core/Character/Components/BP_AttributeComponent.HealthChange` _attributecomponent Damage))
    (:`else`)))

(event `SetEffectsWidget`
  (params (EffectsWidget :type "WidgetComponent Object Reference"))
  ;[1 1 1] Setters
  (set `self.EffectsWidget` EffectsWidget))

(event `SetTimerHealth`
  ;[1 1 1] Health
  (bind _returnvalue (`KismetSystemLibrary.K2_SetTimerDelegate` (delegate `TimerBody`) (`self.TimerDelta`) true))
  (set `self.Timer` _returnvalue))

(event `TimeSum`
  (bind (_settings_attribute _settings_needtimer _settings_time) (break `/Game/Core/Effect/Structure/S_EffectStructure` (`self.Settings`)))
  ;[1 1 1] TimerSum
  (set `self.TimerSum` (`KismetMathLibrary.FClamp` (+ (`self.TimerSum`) (`self.TimerDelta`)) 0.0 _settings_time)))

(event `TimerBody`
  (bind (_settings_attribute _settings_needtimer _settings_time _settings_damage) (break `/Game/Core/Effect/Structure/S_EffectStructure` (`self.Settings`)))
  (bind (_settings_attribute_2 _settings_needtimer_2 _settings_time_2) (break `/Game/Core/Effect/Structure/S_EffectStructure` (`self.Settings`)))
  ;[1 1 1] Health
  (`self.TimeSum`)
  (if (not (== (`self.TimerSum`) _settings_time_2))
    (`self.HealthDamage` _settings_damage)
    (else
      (`self.InvalidedTimer`)
      (`self.RemoveWidget`)
      (`self.OnReadyForDelete` self))))