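; BP_BaseCharacter is a base character that supports attributes and applied effects.
; On BeginPlay it hands the attribute component and effects widget to the effect-handling component, and SetEffect forwards incoming effects to that component.
; Attribute component events drive the rest: speed changes set max walk speed, health changes update the health widget, and expired health destroys the actor through a brief lifespan.
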(event `self.ReceiveBeginPlay`
  (bind _bp_handleeffectcomponent (`self.BP_HandleEffectComponent`))
  ;[1 1 1] Init
  (`/Game/Core/Character/Components/BP_HandleEffectComponent.SetAttributeComponent` _bp_handleeffectcomponent (`self.BP_AttributeComponent`))
  (`/Game/Core/Character/Components/BP_HandleEffectComponent.SetEffectsWidget` _bp_handleeffectcomponent (`self.EffectsWidget`)))

(event `self.BP_AttributeComponent.OnHealthExpired`
  ;[1 1 1] Delete
  (`self.SetLifeSpan` 0.1))

(event `/Game/Core/Character/Interface/BI_SetEffect.SetEffect`
  (params (EffectParam :type "/Game/Core/Effect/Structure/S_EffectStructure Structure"))
  ;[1 1 1] SetEffect
  (`/Game/Core/Character/Components/BP_HandleEffectComponent.SetEffect` (`self.BP_HandleEffectComponent`) EffectParam))

(event `self.BP_AttributeComponent.OnMovementSpeedChange`
  (params (CurrentMovementSpeed :type "Float (single-precision)"))
  ;[1 1 1] SetNewSpeed
  (set `CharacterMovementComponent.MaxWalkSpeed` CurrentMovementSpeed (`self.CharacterMovement`)))

(event `self.BP_AttributeComponent.OnHealthChange`
  (params (CurrentHealth :type "Float (single-precision)"))
  ;[1 1 1] SetNewHealthForWidget
  (message `/Game/Widget/Interface/BI_SetNewPercent.SetNewPercent` (`WidgetComponent.GetWidget` (`self.HealthWidget`)) CurrentHealth))

(fn `UserConstructionScript`)