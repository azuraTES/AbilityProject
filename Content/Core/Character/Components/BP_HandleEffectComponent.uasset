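; BP_HandleEffectComponent is a component that applies effects to its owner by managing a list of active effect objects.
; SetEffect constructs a BP_EffectObject per effect, stores it, passes it the attribute component and effects widget, then activates it with the given setting.
; It binds to each object's ready-for-delete event, with a handler that removes objects from the array.
; Setters supply the attribute component and widget references.
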(event `SetEffect`
  (params (EffectSetting :type "/Game/Core/Effect/Structure/S_EffectStructure Structure"))
  ;[1 1 1] CreateAndAddToArray
  (bind _returnvalue (`|GenericCreateObject` "/Game/Core/Effect/BP_EffectObject.BP_EffectObject_C" (`self.GetOwner`)))
  (`KismetArrayLibrary.Array_Add` (`self.EffectsObject`) _returnvalue)
  ;[1 1 1] InitComp
  (`/Game/Core/Effect/BP_EffectObject.SetAttributeComponent` _returnvalue (`self.AttributeComponent`))
  (`/Game/Core/Effect/BP_EffectObject.SetEffectsWidget` _returnvalue (`self.EffectsWidget`))
  (`/Game/Core/Effect/BP_EffectObject.ActivateEffect` _returnvalue EffectSetting)
  (add `/Game/Core/Effect/BP_EffectObject.OnReadyForDelete` _returnvalue (`|CreateDelegate` :!event `DeleteObjectFromArray`)))

(event `DeleteObjectFromArray`
  (params (Object :type "Object Object Reference"))
  ;[1 1 1] DeleteEffectObject
  (`KismetArrayLibrary.Array_RemoveItem` (`self.EffectsObject`) Object))

(event `SetAttributeComponent`
  (params (AttributeComponent :type "/Game/Core/Character/Components/BP_AttributeComponent Object Reference"))
  ;[1 1 1] Setters
  (set `self.AttributeComponent` AttributeComponent))

(event `SetEffectsWidget`
  (params (EffectsWidget :type "WidgetComponent Object Reference"))
  ;[1 1 1] Setters
  (set `self.EffectsWidget` EffectsWidget))