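; BP_AttributeComponent is a character component that tracks Health and MovementSpeed attributes.
; Each has a change event that subtracts a Damage amount, calling an OnChange dispatcher, or only OnExpired when the value hits zero.
; Changes are ignored once the value is zero, until a reset event restores the maximum and broadcasts the change.
; Values are not clamped to their maximum, and BeginPlay and Tick are unused.
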(event `HealthChange`
  (params (Damage :type "Float (double-precision)"))
  (bind _returnvalue (- (`self.Health`) Damage))
  (if (!= (`self.Health`) 0.0)
    (if (<= _returnvalue 0.0)
      (set `self.Health` 0.0)
      (`self.OnHealthExpired`)
      (else
        (bind _output_get (set `self.Health` _returnvalue))
        (`self.OnHealthChange` _output_get)))))

(event `ResetHealth`
  ;[1 1 1] Reset
  (bind _output_get (set `self.Health` (`self.MaxHealth`)))
  (`self.OnHealthChange` _output_get))

(event `MovementSpeedChange`
  (params (Damage :type "Float (double-precision)"))
  (bind _returnvalue (- (`self.MovementSpeed`) Damage))
  (if (!= (`self.MovementSpeed`) 0.0)
    (if (<= _returnvalue 0.0)
      (set `self.MovementSpeed` 0.0)
      (`self.OnMovementSpeedExpired`)
      (else
        (bind _output_get (set `self.MovementSpeed` _returnvalue))
        (`self.OnMovementSpeedChange` _output_get)))))

(event `ResetMovementSpeed`
  ;[1 1 1] Reset
  (bind _output_get (set `self.MovementSpeed` (`self.MaxMovementSpeed`)))
  (`self.OnMovementSpeedChange` _output_get))