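; BP_PlayerCharacter is the player character Blueprint, which equips and fires a first-person weapon.
; On BeginPlay it spawns a BP_Weapon owned by itself and snaps it to the skeletal mesh's GripPoint socket.
; Its Fire event plays the first-person fire montage on that mesh, then passes the InputID to the weapon's own Fire.
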(event `self.ReceiveBeginPlay`
  (`parent.ReceiveBeginPlay`)
  (`self.CreateAndInitWeapon`))

(event `CreateAndInitWeapon`
  ;[1 1 1] InitWeapon
  (bind _returnvalue (`|SpawnActorFromClass` "/Game/Core/Weapon/BP_Weapon.BP_Weapon_C" (`self.GetTransform`) "AlwaysSpawn" "OverrideRootScale" self null))
  (bind _output_get (set `self.BP_Weapon` _returnvalue))
  (`SceneComponent.K2_AttachToComponent` (`Actor.RootComponent` _output_get) (`self.SkeletalMesh`) "GripPoint" "SnapToTarget" "SnapToTarget" "SnapToTarget" true))

(event `Fire`
  (params (InputID :type "/Game/Core/Effect/Enum/E_InputID Enum" :default "NewEnumerator0"))
  ;[1 1 1] Fire
  (`AnimInstance.Montage_Play` (`SkeletalMeshComponent.GetAnimInstance` (`self.SkeletalMesh`)) "/Game/FirstPerson/Animations/FirstPersonFire_Montage.FirstPersonFire_Montage" 1.0 "MontageLength" 0.0 true)
  (`/Game/Core/Weapon/BP_Weapon.Fire` (`self.BP_Weapon`) InputID))

(fn `UserConstructionScript`)