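; BP_Weapon is a weapon actor that fires projectiles from its skeletal mesh.
; Its Fire event spawns a BP_Projectile, passing along an InputID, and plays a firing sound at the weapon's location.
; A helper function builds the spawn transform from the Muzzle socket, adding GunOffset rotated into the socket's orientation.
; Spawning adjusts around collisions and fails if the projectile would still overlap.
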(event `Fire`
  (params (InputID :type "/Game/Core/Effect/Enum/E_InputID Enum" :default "NewEnumerator0"))
  (`|SpawnActorFromClass` "/Game/Core/Weapon/Projectile/BP_Projectile.BP_Projectile_C" (`self.MakeTransormForProjectile`) "AdjustIfPossibleButDontSpawnIfColliding" "OverrideRootScale" null InputID null) ; Spawn projectile
  (`GameplayStatics.PlaySoundAtLocation` "/Game/FirstPerson/Audio/FirstPersonTemplateWeaponFire02.FirstPersonTemplateWeaponFire02" (`self.K2_GetActorLocation`) (struct) 1.0 1.0 0.0 null null null) ; Play firing sound
)

(fn `MakeTransormForProjectile`
  (returns (ReturnValue :type "Transform Structure"))
  (bind _returnvalue (`SceneComponent.GetSocketRotation` (`self.SkeletalMesh`) (`self.Muzzle`)))
  (return (`KismetMathLibrary.MakeTransform` (+ (`SceneComponent.GetSocketLocation` (`self.SkeletalMesh`) (`self.Muzzle`)) (`KismetMathLibrary.GreaterGreater_VectorRotator` (`self.GunOffset`) _returnvalue)) _returnvalue)))

(fn `UserConstructionScript`)